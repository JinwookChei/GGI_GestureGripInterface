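; BP_GGIPawn is a VR pawn that records hand motion capture data to CSV.
; On BeginPlay, if a head-mounted display is enabled, it sets a Stage tracking origin and fixes VR pixel density through a console command.
; Pressing F initializes HandMotionCaptureComponent with both XR controllers and hands, then, if that succeeds, starts CSV writing with a hardcoded Pistol argument.
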(event EventBeginPlay
  (if (Class|HeadMountedDisplayFunctionLibrary|IsHeadMountedDisplayEnabled)
    (Class|HeadMountedDisplayFunctionLibrary|SetTrackingOrigin "Stage")
    (Development|ExecuteConsoleCommand "vr.PixelDensity 1.0" 0)))

(event Collision|EventActorBeginOverlap
  (params (OtherActor :type Actor%20Object%20Reference)))

(event EventTick
  (params (DeltaSeconds :type Float%20%28single-precision%29)))

(event Input|KeyboardEvents|F
  (params (Key :type Key%20Structure :default "None"))
  (bind _handmotioncapturecomponent (Variables|Default|GetHandMotionCaptureComponent))
  (:Pressed
    (bind _returnvalue (Class|HandMotionCaptureComponent|Initialize _handmotioncapturecomponent (Variables|Default|GetRightXRController) (Variables|Default|GetLeftXRController) (Variables|Default|GetRightXRHand) (Variables|Default|GetLeftXRHand)))
    (if _returnvalue
      (Class|HandMotionCaptureComponent|StartWriteCSVData _handmotioncapturecomponent "Pistol"))))

(fn ConstructionScript)